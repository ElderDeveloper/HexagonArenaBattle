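; Hex grid manager Blueprint whose event graph holds debug demos for random tile selection and pathfinding.
; A custom event picks two random hex tiles, finds a path between them, and draws colored spheres and step indices along it.
; Grid queries and pathfinding are called functions not defined in these graphs.
; Unconnected demos show neighbor lookup and random tile locations; the construction script is empty.
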(event `CustomEvent`
  ; Demo For Random Hex Tile And Path Generation
  (bind _output_get (set `self.RandomHex` (`self.GetRandomHexTile`)))
  (`KismetSystemLibrary.DrawDebugSphere` (`self.K2_GetActorLocation` _output_get) 50.0 12 (struct :`R` 0.651062 :`G` 1.0 :`A` 1.0) 3.0 1.0)
  (bind _output_get_2 (set `self.RandomHex2` (`self.GetRandomHexTile`)))
  (`KismetSystemLibrary.DrawDebugSphere` (`self.K2_GetActorLocation` _output_get_2) 50.0 12 (struct :`G` 0.41843 :`B` 1.0 :`A` 1.0) 3.0 1.0)
  (bind _output_get_3 (set `self.Path` (`self.FindPathWithTiles` (`self.RandomHex`) (`self.RandomHex2`))))
  (for (_array_element _array_index) _output_get_3
    (bind _returnvalue (`self.K2_GetActorLocation` _array_element))
    (`KismetSystemLibrary.DrawDebugSphere` _returnvalue 30.0 12 (struct :`R` 1.0 :`G` 0.014881 :`A` 1.0) 3.0 1.0)
    (`KismetSystemLibrary.DrawDebugString` _returnvalue (`KismetStringLibrary.Conv_IntToString` _array_index) null (struct :`R` 1.0 :`G` 1.0 :`B` 1.0 :`A` 1.0) 3.0)))

(fn `UserConstructionScript`)